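; BP_LOPanel is a clickable sprite panel that flips between lit and unlit and fades in and out.
; Clicking the sprite calls OnClickPanel, while Flip and Fade either snap instantly or play timelines forward or backward, calling OnFliped or OnFaded when finished.
; Both drive one sprite color: SetEmissive blends normal and emissive colors while keeping alpha, and SetOpacity changes only alpha.
; Construction starts it unlit and transparent.
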(event OnClicked(SpriteComponent)
  (params (TouchedComponent :type Primitive%20Component%20Object%20Reference) (ButtonPressed :type Key%20Structure :default "None"))
  ;[1 1 1] クリックイベント
  (Class|LOPanel|OnClickPanel))

(event EventFlip
  (params (IsLight :type Boolean) (IsSkip :type Boolean))
  ;[1 1 1] 色を反転させる
  (if IsSkip ; アニメーションをスキップ
    (if IsLight ; ON/OFF
      (CallFunction|SetEmissive 1.0)
      (else
        (CallFunction|SetEmissive 0.0)))
    (else
      ;;[1 1 1] フェードアニメーション
      (if IsLight ; ON/OFF
        (bind _changelight (Timeline|ChangeLightTimeline PlayFromStart)
          (:Update
            (CallFunction|SetEmissive _changelight))
          (:Finished
            (Class|LOPanel|OnFliped)))
        (else
          (Timeline|ChangeLightTimeline ReverseFromEnd))))))

(event EventFade
  (params (IsShow :type Boolean) (IsSkip :type Boolean))
  ;[1 1 1] フェード
  (if IsSkip ; アニメーションをスキップ
    (if IsShow ; ON/OFF
      (CallFunction|SetOpacity 1.0)
      (else
        (CallFunction|SetOpacity 0.0)))
    (else
      ;;[1 1 1] フェードアニメーション
      (if IsShow
        (bind _panelfade (Timeline|FadeTimeline PlayFromStart)
          (:Update
            (CallFunction|SetOpacity _panelfade))
          (:Finished
            (Class|LOPanel|OnFaded)))
        (else
          (Timeline|FadeTimeline ReverseFromEnd))))))

(fn ConstructionScript
  (CallFunction|SetEmissive 0.0)
  (CallFunction|SetOpacity 0.0))

(fn SetEmissive
  (params (emisive :type Float%20%28double-precision%29))
  (bind _output_get (Variables|Default|SetSpriteColor (Class|KismetMathLibrary|LinearColortoNewOpacity (+ (* (LocalVariables|GetNormalColor) (- 1.0 emisive)) (* emisive (LocalVariables|GetEmissiveColor))) (.a (Variables|Default|GetSpriteColor)))))
  (Sprite|SetSpriteColor (Variables|Default|GetSpriteComponent) _output_get))

(fn SetOpacity
  (params (Opacity :type Float%20%28double-precision%29))
  (bind _output_get (Variables|Default|SetSpriteColor (Class|KismetMathLibrary|LinearColortoNewOpacity (Variables|Default|GetSpriteColor) Opacity)))
  (Sprite|SetSpriteColor (Variables|Default|GetSpriteComponent) _output_get))